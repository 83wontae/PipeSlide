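; BP_MoveBall is a ball actor that gets pushed along pipe splines it touches.
; Every tick it finds the BP_PipeSpline actors overlapping its Sphere component.
; For each, it applies a physics impulse to the Sphere along the spline direction closest to the ball's location, scaled by a fixed strength.
; That direction is read in the spline's local space, while the impulse applies in world space.
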(event `self.ReceiveTick`
  (params (DeltaSeconds :type "Float (single-precision)"))
  (for _array_element (`PrimitiveComponent.GetOverlappingActors` (`self.Sphere`) "/Game/PipeSlide/BP_PipeSpline.BP_PipeSpline_C")
    (bind _asbp_pipe_spline (cast `/Game/PipeSlide/BP_PipeSpline` _array_element))
    (`PrimitiveComponent.AddImpulse` (`self.Sphere`) (* (`SplineComponent.FindDirectionClosestToWorldLocation` (`/Game/PipeSlide/BP_PipeSpline.Spline` _asbp_pipe_spline) (`SceneComponent.K2_GetComponentLocation` (`self.Sphere`)) "Local") 3000.0) "None" false)))

(fn `UserConstructionScript`)